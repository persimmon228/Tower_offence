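; BP_TowerPawn is an enemy turret tower that shoots at the player's tank and can trigger the win screen.
; Range overlaps with BP_TankPawn toggle a flag that makes Tick pass the player's location to AIPlayerShooting.
; Fire uses a call counter to throttle projectile spawns, and BeginPlay tints base and turret through dynamic team-color materials.
; GameResultat spawns an explosion, then shows the win widget and sounds if TowerCheck passes.
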(event OnComponentBeginOverlap(Range)
  (params (OverlappedComponent :type Primitive%20Component%20Object%20Reference) (OtherActor :type Actor%20Object%20Reference) (OtherComp :type Primitive%20Component%20Object%20Reference) (OtherBodyIndex :type Integer) (bFromSweep :type Boolean) (SweepResult :type Hit%20Result%20Structure%20%28by%20ref%29))
  (Utilities|Casting|CastToBP_TankPawn OtherActor)
  (Variables|Default|SetIneedOverlapingTick 1))

(event OnComponentEndOverlap(Range)
  (params (OverlappedComponent :type Primitive%20Component%20Object%20Reference) (OtherActor :type Actor%20Object%20Reference) (OtherComp :type Primitive%20Component%20Object%20Reference) (OtherBodyIndex :type Integer))
  (Utilities|Casting|CastToBP_TankPawn OtherActor)
  (Variables|Default|SetIneedOverlapingTick 0))

(event Custom|Change%20color
  (params (NewParam :type Static%20Mesh%20Component%20Object%20Reference))
  (bind _returnvalue (Rendering|Material|CreateDynamicMaterialInstance NewParam 1 (Rendering|Material|GetMaterial NewParam 1) "None" :!class /Script/Engine.PrimitiveComponent))
  (Rendering|Material|SetVectorParameterValue _returnvalue "TeamColor" (Variables|Default|GetTeam%20Color) :!class /Script/Engine.MaterialInstanceDynamic))

(event EventBeginPlay
  (CallFunction|ChangeColor (Variables|Default|GetMyBaseMesh))
  (CallFunction|ChangeColor (Variables|Default|GetMyTurretMesh)))

(event Collision|EventActorBeginOverlap
  (params (OtherActor :type Actor%20Object%20Reference)))

(event EventTick
  (params (DeltaSeconds :type Float%20%28single-precision%29))
  (if (== (Variables|Default|GetIneedOverlapingTick) 1)
    (Class|TowerPawn|AIPlayerShooting (Transformation|GetActorLocation (Game|Player|GetPlayerPawn 0)))))

(event EventGameResultat
  (Effects|SpawnEmitteratLocation "/Game/Realistic_Starter_VFX_Pack_Vol2/Particles/Explosion/P_Explosion_Big_A.P_Explosion_Big_A" (Transformation|GetActorLocation))
  (bind _returnvalue (Class|TowerPawn|TowerCheck))
  (if _returnvalue
    (bind _returnvalue_2 (UserInterface|CreateWidget "/Game/UI/Win.Win_C"))
    (UserInterface|Viewport|AddtoViewport _returnvalue_2 0)
    (Audio|PlaySound2D "/Game/Sounds/Win_Wave.Win_Wave" 1.0 1.0 0.0 0 0)
    (Audio|PlaySound2D "/Game/Sounds/Win_Voice_Wave.Win_Voice_Wave" 1.0 1.0 0.0 0 0)))

(fn ConstructionScript)

(fn Fire
  (if (== 3 (Variables|Default|Gettimer))
    (Variables|Default|Settimer 0)
    (Game|SpawnActorfromClass "/Game/Blueprints/BP_Projectile.BP_Projectile_C" (Math|Transform|MakeTransform (Transformation|GetWorldLocation (Variables|Default|GetMyProjectileSpawnPoint)) (Transformation|GetSocketRotation (Variables|Default|GetMyProjectileSpawnPoint) "None") "1.000000,1.000000,1.000000") "Undefined" "MultiplyWithRoot" 0 (Game|Player|GetPlayerPawn 0))
    (else
      (Math|Integer|IncrementInt (Variables|Default|Gettimer)))))