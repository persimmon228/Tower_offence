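; BP_TankPawn is a player-controlled tank pawn using Enhanced Input.
; BeginPlay adds its mapping context, and the TurnAround action feeds controller yaw and pitch for mouse camera control.
; Move applies forward movement input, and Turn sets world roll on base, turret and projectile spawn point, zeroing pitch and yaw.
; The MoveForward event is empty, and nothing in the graph calls Move or Turn.
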(event Input|EnhancedActionEvents|EnhancedInputActionMoveForward
  (params (ActionValue :type Float%20%28double-precision%29) (ElapsedSeconds :type Float%20%28double-precision%29) (TriggeredSeconds :type Float%20%28double-precision%29) (InputAction :type Input%20Action%20Object%20Reference :default "/Game/Inputs/Input_Actions/MoveForward.MoveForward"))
  ;[1 1 1] All Tank Moving
)

(event Input|EnhancedActionEvents|EnhancedInputActionTurnAround
  (params (ActionValue :type Vector%202D%20Structure) (ElapsedSeconds :type Float%20%28double-precision%29) (TriggeredSeconds :type Float%20%28double-precision%29) (InputAction :type Input%20Action%20Object%20Reference :default "/Game/Inputs/Input_Actions/TurnAround.TurnAround"))
  ;[1 1 1] Mouse Camera moving
  (Pawn|Input|AddControllerYawInput (.x ActionValue))
  (Pawn|Input|AddControllerPitchInput (.y ActionValue)))

(event EventBeginPlay
  ;[1 1 1] Add inputs control
  (bind _asplayer_controller (Utilities|Casting|CastToPlayerController (Pawn|GetController)))
  (Utilities|IsValid (PlayerController|LocalPlayerSubsystems|GetEnhancedInputLocalPlayerSubsystem _asplayer_controller)
    (:Is%20Valid
      (Input|AddMappingContext (PlayerController|LocalPlayerSubsystems|GetEnhancedInputLocalPlayerSubsystem _asplayer_controller) "/Game/Inputs/Inputs_maps/Map_context.Map_context" 0 "(bIgnoreAllPressedKeysUntilRelease=True,bForceImmediately=False,bNotifyUserSettings=False)"))))

(event Collision|EventActorBeginOverlap
  (params (OtherActor :type Actor%20Object%20Reference)))

(event EventTick
  (params (DeltaSeconds :type Float%20%28single-precision%29)))

(fn ConstructionScript)

(fn Move
  (params (DistansToMove :type Float%20%28single-precision%29))
  (Pawn|Input|AddMovementInput (Transformation|GetActorForwardVector) DistansToMove false))

(fn Turn
  (params (Rotation :type Float%20%28single-precision%29))
  (Transformation|SetWorldRotation (Variables|Default|GetMyBaseMesh) (Math|Rotator|MakeRotator Rotation 0.0 0.0) false false))