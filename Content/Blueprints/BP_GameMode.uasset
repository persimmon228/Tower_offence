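; Game mode for a tank game that recolors tanks with one of four team colors.
; ChangeColor selects a BP_TankPawn by its index in GetAllActorsOfClass and passes its turret and base meshes to ColorHelper.
; ColorHelper creates a dynamic material instance on material slot 1 and sets its TeamColor parameter from the color index.
; The event graph holds no active logic.
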(event EventBeginPlay)

(event EventTick
  (params (DeltaSeconds :type Float%20%28single-precision%29)))

(fn ConstructionScript)

(fn ChangeColor
  (params (color :type Integer) (Tank :type Integer))
  (bind _outactors (Actor|GetAllActorsOfClass "/Game/Blueprints/BP_TankPawn.BP_TankPawn_C"))
  (for (_array_element _array_index) _outactors
    (if (== Tank _array_index)
      (CallFunction|ColorHelper color (Variables|/Script/Tower_offence.TurrentPawn|GetMyTurretMesh _array_element) (Rendering|Material|GetMaterial (Variables|/Script/Tower_offence.TurrentPawn|GetMyTurretMesh _array_element) 1))
      (CallFunction|ColorHelper color (Variables|/Script/Tower_offence.TurrentPawn|GetMyBaseMesh _array_element) (Rendering|Material|GetMaterial (Variables|/Script/Tower_offence.TurrentPawn|GetMyBaseMesh _array_element) 1)))))

(fn ColorHelper
  (params (Color :type Integer) (Mesh :type Primitive%20Component%20Object%20Reference) (Material :type Material%20Interface%20Object%20Reference))
  (bind _returnvalue (Rendering|Material|CreateDynamicMaterialInstance Mesh 1 Material "None" :!class /Script/Engine.PrimitiveComponent))
  (if (== Color 0)
    (Rendering|Material|SetVectorParameterValue _returnvalue "TeamColor" (Variables|Default|Getcolor%201) :!class /Script/Engine.MaterialInstanceDynamic)
    (elif (== Color 1)
      (Rendering|Material|SetVectorParameterValue _returnvalue "TeamColor" (Variables|Default|GetColor%202) :!class /Script/Engine.MaterialInstanceDynamic)
      (elif (== Color 2)
        (Rendering|Material|SetVectorParameterValue _returnvalue "TeamColor" (Variables|Default|GetColor%203) :!class /Script/Engine.MaterialInstanceDynamic)
        (else
          (Rendering|Material|SetVectorParameterValue _returnvalue "TeamColor" (Variables|Default|GetColor%204) :!class /Script/Engine.MaterialInstanceDynamic))))))